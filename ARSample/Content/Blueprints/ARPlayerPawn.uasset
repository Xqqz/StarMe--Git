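; AR player pawn that places objects on detected real-world planes at the touched screen point, branching between ARCore on Android and ARKit otherwise.
; Android line-traces the deprojected touch against planes and spawns an anchor placeable tied to the hit plane; iOS hit-tests existing planes and spawns a plain placeable.
; Each tick prints camera transform and tracking quality, downgrading Normal to Limited until ARCore finds a plane; ARKit assumes one exists.
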(event EventBeginPlay
  (CallFunction|CachePlatform))

(event EventTick
  (params (DeltaSeconds :type Float%20%28single-precision%29))
  ;[0 0 0] Display Debug Information About Found Planes
  (Utilities|FlowControl|Sequence
    (:then_0
      (if (Variables|Default|GetbIsAndroid)
        ;;[0.5145 1 0.2552 0.3] ARCore : takes a while to detect the first plane, so incorporate this info into tracking quality reporting
        (CallFunction|FindPlanesforARCORE)
        (else
          ;;[0.156 0.5013 1 0.3] ARKit : detects planes quickly enough to just assume it found one if the tracking is good
          (Variables|Default|SetnumPlanesDetected 1))))
    (:then_1
      (CallFunction|DisplayDebugTrackingInfo))))

(event Input|TouchEvents|InputTouch
  (params (Location :type Vector) (FingerIndex :type ETouchIndex%20Enum))
  (bind _returnvalue (Game|GetPlayerController 0))
  (bind (_locationx _locationy) (Class|PlayerController|GetInputTouchState _returnvalue FingerIndex))
  (bind _returnvalue_2 (Math|Vector2D|MakeVector2D _locationx _locationy))
  (:Pressed
    ;[0 0 0] ARCore and ARKit currently have differences in plane detection as well as how they expect Actors to be placed in the world, so we account for that here. Expect updates that simplify this in future releases
    (if (Variables|Default|GetbIsAndroid)
      ;;[0.5145 1 0.2552 0.3] Android Path
      (bind (_success _spawntransform _plane) (CallFunction|DoHitTestforARCORE _returnvalue _returnvalue_2))
      (if _success
        (bind _returnvalue_3 (Game|SpawnActorfromClass "/Game/Blueprints/BP_GoogleAnchorPlaceable.BP_GoogleAnchorPlaceable_C" _spawntransform "AlwaysSpawn" 0 0))
        (Variables|/Game/Blueprints/BP_GoogleAnchorPlaceable.BP_GoogleAnchorPlaceable_C|SetAttachedPlane _returnvalue_3 _plane)
        (else
          ;[1 -0.7571 -1.971] No Hit Info Found
          (Development|PrintString (Utilities|String|Append "NO HIT" (Utilities|String|ToString(Vector2d) _returnvalue_2)) true true "(R=1.000000,G=0.000000,B=0.356152,A=1.000000)" 1.0 :!label _label)))
      (else
        ;;[0.156 0.5013 1 0.3] iOS Path
        (bind (_success_2 _spawntransform_2) (CallFunction|DoHitTestforARKIT _returnvalue_2))
        (if _success_2
          (Game|SpawnActorfromClass "/Game/Blueprints/BP_Placeable.BP_Placeable_C" _spawntransform_2 "AlwaysSpawn" 0 0)
          (else
            (goto _label)))))))

(fn ConstructionScript)

(fn DetermineTrackingQuality
  (bind _returnvalue (Class|ARBlueprintFunctionLibrary|GetTrackingQuality))
  ;[1 1 1] If we haven't found any planes yet, downgrade the tracking quality by 1 notch.
  (bind _output_get (LocalVariables|SetTrackingQuality _returnvalue))
  (return (select (>= (Variables|Default|GetnumPlanesDetected) 1) _output_get (Utilities|Select :Index _output_get :NotAvailable "NotAvailable" :Limited "Limited" :Normal "Limited"))))

(fn DoHitTestforARCORE
  (params (Player :type Player%20Controller%20Object%20Reference) (InputPin :type Vector%202D%20Structure))
  (bind (_worldposition _worlddirection) (Class|GameplayStatics|DeprojectScreentoWorld Player InputPin))
  (bind (_impactpoint _impactnormal _outplaneobject _returnvalue) (Class|GoogleARCoreSessionFunctionLibrary|LineTraceSingleonPlanes _worldposition (+ _worldposition (* _worlddirection 1e+04)) false))
  (if _returnvalue
    (Development|PrintString (Utilities|String|Append "HIT from :  " (Utilities|String|ToString(Vector2d) InputPin)) true true "(R=0.707400,G=1.000000,B=0.000000,A=1.000000)")
    (Development|PrintString (Utilities|String|ToString(Transform) (Math|Transform|MakeTransform _impactpoint)) true true "(R=1.000000,G=0.965410,B=0.000000,A=1.000000)")
    (return true (Math|Transform|MakeTransform _impactpoint) _outplaneobject)
    (else
      (return false "" 0))))

(fn DoHitTestforARKIT
  (params (InputPin :type Vector%202D%20Structure))
  (bind (_outresults _returnvalue) (Class|AppleARKitBlueprintLibrary|HitTestatScreenPositionTrackingSpace InputPin "ExistingPlane"))
  (if _returnvalue
    (Development|PrintString (Utilities|String|Append "HIT from :  " (Utilities|String|ToString(Vector2d) InputPin) " Distance : " (Utilities|String|ToString(Float) (.Distance (Utilities|Struct|BreakAppleARKitHitTestResult (Utilities|Array|Get(acopy) _outresults))))) true true "(R=0.707400,G=1.000000,B=0.000000,A=1.000000)")
    (Development|PrintString (Utilities|String|ToString(Transform) (.Transform (Utilities|Struct|BreakAppleARKitHitTestResult (Utilities|Array|Get(acopy) _outresults)))) true true "(R=1.000000,G=0.965410,B=0.000000,A=1.000000)")
    (return true (.Transform (Utilities|Struct|BreakAppleARKitHitTestResult (Utilities|Array|Get(acopy) _outresults))))
    (else
      (return false ""))))

(fn CachePlatform
  ;[1 1 1] Cache platform that we're running on for switching on platform-specific functionality
  (bind _returnvalue (Game|GetPlatformName))
  (bind _output_get (Variables|Default|SetbIsAndroid (Utilities|Enum|Equal(Enum) _returnvalue "Android")))
  (Development|PrintString _returnvalue)
  (Development|PrintString (Utilities|String|ToString(Boolean) _output_get)))

(fn DisplayDebugTrackingInfo
  ;[1 1 1] Display Debug Tracking Info
  (Development|PrintString (Utilities|String|ToString(Transform) (Transformation|GetWorldTransform (Variables|/Script/Engine.PlayerCameraManager|GetTransformComponent (Game|GetPlayerCameraManager 0)))) true false "(R=0.081168,G=1.000000,B=0.218801,A=1.000000)" 0.0)
  (bind _tracking (CallFunction|DetermineTrackingQuality))
  (Development|PrintString (Utilities|String|Append "[ " (Utilities|String|EnumtoString _tracking) " ]") true false (Utilities|Select :Index _tracking :NotAvailable "(R=1.000000,G=0.000000,B=0.158961,A=1.000000)" :Limited "(R=1.000000,G=0.226966,B=0.000000,A=1.000000)" :Normal "(R=0.283149,G=1.000000,B=0.000000,A=1.000000)") 0.0))

(fn FindPlanesforARCORE
  (bind _outarcoreplanelist (Class|GoogleARCoreFrameFunctionLibrary|GetAllPlanes))
  (Development|PrintString (Utilities|String|ToString(Integer) (Utilities|Array|Length _outarcoreplanelist)) true false "(R=0.000000,G=0.660000,B=1.000000,A=1.000000)" 0.0)
  (Variables|Default|SetnumPlanesDetected (Utilities|Array|Length _outarcoreplanelist)))